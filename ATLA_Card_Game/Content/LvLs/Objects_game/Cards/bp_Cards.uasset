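; Card helper Blueprint that provides shared functions for drawing random cards and animating card widgets.
; Two getters pick a random entry from a deck's attack card or defense card array.
; An interpolation helper eases a widget transform's translation and angle toward a destination using delta time and a given speed, leaving scale and shear at defaults.
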(fn `getRandomAttackCard`
  (params (Deck :type "/Game/LvLs/Objects_game/Decks/Deck Structure"))
  (returns (cardInfo :type "/Game/LvLs/Objects_game/Cards/CardAtackStructure Structure"))
  (return (`KismetArrayLibrary.Array_Random` (`.Attackcards_3_D3BFB84B4AD0E6EF09597DA300C25CEE` (break `/Game/LvLs/Objects_game/Decks/Deck` Deck)))))

(fn `getRandomDeffCard`
  (params (DeckCards :type "/Game/LvLs/Objects_game/Decks/Deck Structure"))
  (returns (cardInfo :type "/Game/LvLs/Objects_game/Cards/CardDefStructure Structure"))
  (return (`KismetArrayLibrary.Array_Random` (`.Deffcards_6_D236A7E247B17D71CCC2DDBD42D13000` (break `/Game/LvLs/Objects_game/Decks/Deck` DeckCards)))))

(fn `interploateTowardPostions`
  (params (CurrentPostion :type "WidgetTransform Structure") (DestinationTransform :type "WidgetTransform Structure") (delta :type "Float (double-precision)") (InterpolationSpeed :type "Float (double-precision)"))
  (returns (NewPostion :type "WidgetTransform Structure"))
  (bind (_translation _scale _shear _angle) (break `WidgetTransform` CurrentPostion))
  (bind (_translation_2 _scale_2 _shear_2 _angle_2) (break `WidgetTransform` DestinationTransform))
  (bind _delta (`local.delta`))
  (bind _interpolationspeed (`local.InterpolationSpeed`))
  (return (make `WidgetTransform` (`KismetMathLibrary.Vector2DInterpTo` _translation _translation_2 _delta _interpolationspeed) (1.0 1.0) (0.0 0.0) (`KismetMathLibrary.FInterpTo` _angle _angle_2 _delta _interpolationspeed))))